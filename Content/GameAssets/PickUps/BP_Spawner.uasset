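; BP_Spawner is a pickup spawner actor that places one randomly chosen object inside a box area.
; On BeginPlay, only the authority starts a short one-shot timer, which calls Spawn.
; Spawn picks a random class from SpawnableObjects and creates it at a random point within the scaled SpawnArea extents, centered on the actor's location.
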(event `self.ReceiveBeginPlay`
  (`/Engine/EditorBlueprintResources/ActorMacros.Switch Has Authority`
    (:`Authority`
      (`KismetSystemLibrary.K2_SetTimerDelegate` (delegate `Timer`) 1.0))))

(event `Timer`
  (`self.Spawn`))

(fn `Spawn`
  (locals (SpawnableObjects :type "Array of Actor Class Reference"))
  (`|SpawnActorFromClass` (`KismetArrayLibrary.Array_Random` (`local.SpawnableObjects`)) (`KismetMathLibrary.MakeTransform` (`KismetMathLibrary.RandomPointInBoundingBox` (`self.K2_GetActorLocation`) (`BoxComponent.GetScaledBoxExtent` (`self.SpawnArea`)))) "Undefined" "MultiplyWithRoot" null null))

(fn `UserConstructionScript`)